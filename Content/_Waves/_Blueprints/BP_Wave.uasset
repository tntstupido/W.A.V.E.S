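; BP_Wave is a wave actor that gives its mesh a random color when play begins.
; BeginPlay creates a dynamic material instance, then UpdateWaveColor picks Blue, Red, Yellow or Green at random.
; It looks that frequency up in the color set from BP_GM_Waves and writes the color to the BaseColor parameter.
; Actor overlaps only print the other actor's name.
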(event EventBeginPlay
  (Utilities|FlowControl|Sequence
    (:then_0
      (bind _returnvalue (Rendering|Material|CreateDynamicMaterialInstance (Variables|Character|GetMesh) 0 0 "None" :!class /Script/Engine.PrimitiveComponent))
      (Variables|Default|SetWaveDMI _returnvalue))
    (:then_1
      (CallFunction|UpdateWaveColor))))

(event Collision|EventActorBeginOverlap
  (params (OtherActor :type Actor%20Object%20Reference))
  (Development|PrintString (Utilities|GetDisplayName OtherActor)))

(fn ConstructionScript)

(fn UpdateWaveColor
  (Variables|Default|GetWaveDMI
    (:then
      (bind _asbp_gm_waves (Utilities|Casting|CastToBP_GM_Waves (Game|GetGameMode)))
      (Rendering|Material|SetVectorParameterValue (Variables|Default|GetWaveDMI) "BaseColor" (.Color (Utilities|Struct|BreakWaveColorDef (Class|DAWaveColorSet|FindbyFrequency (Class|GMWaves|GetColorSet _asbp_gm_waves) (.OutItem (Utilities|Array|Random (Utilities|Array|MakeArray "Blue" "Red" "Yellow" "Green")))))) :!class /Script/Engine.MaterialInstanceDynamic))
    (:else)))