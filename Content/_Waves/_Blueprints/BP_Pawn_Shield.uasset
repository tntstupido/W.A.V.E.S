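; BP_Pawn_Shield is a pawn shield Blueprint that tints its shield mesh to match the shield's current frequency.
; On BeginPlay it creates a dynamic material instance from the shield mesh.
; When the Shield component reports a frequency change, it looks up that frequency's color in the BP_GM_Waves game mode's color set and writes it to the material's FrequencyColor parameter.
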(event OnFrequencyChanged(Shield)
  (params (NewFreq :type EWaveFrequency%20Enum :default "Blue"))
  (Variables|Default|GetShieldDMI
    (:then
      (bind _asbp_gm_waves (Utilities|Casting|CastToBP_GM_Waves (Game|GetGameMode)))
      (Rendering|Material|SetVectorParameterValue (Variables|Default|GetShieldDMI) "FrequencyColor" (.Color (Utilities|Struct|BreakWaveColorDef (Class|DAWaveColorSet|FindbyFrequency (Class|GMWaves|GetColorSet _asbp_gm_waves) NewFreq))) :!class /Script/Engine.MaterialInstanceDynamic))
    (:else)))

(event EventBeginPlay
  (Utilities|FlowControl|Sequence
    (:then_0
      (bind _returnvalue (Rendering|Material|CreateDynamicMaterialInstance (Variables|Default|GetShieldMesh) 0 0 "None" :!class /Script/Engine.PrimitiveComponent))
      (Variables|Default|SetShieldDMI _returnvalue))))

(fn ConstructionScript)